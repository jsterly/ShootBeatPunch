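; SoundMaster plays the level song from GameManager and drives the beat state and level countdown from it.
; Playback percent gives the played time, which indexes Constant-Q analysis to set the character's CharOnBeat and pulse two glow parameter collections.
; Tick updates TimeRemaining, pauses audio while the character's Timer runs, and lowers pitch in steps as IpodBurnout rises.
; When time runs out, it banks level currency and opens the Commissary.
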(event `self.ReceiveBeginPlay`
  (bind _returnvalue (`GameplayStatics.GetPlayerController` 0))
  (bind _audio (`self.Audio`))
  (bind _audio_2 (`self.Audio`))
  (bind _asgame_manager (cast `/Game/GameManager` (`GameplayStatics.GetGameInstance`)))
  (bind _mainsound (`/Game/GameManager.MainSound` _asgame_manager))
  (`AudioComponent.SetSound` (`self.Audio`) _mainsound)
  (set `self.Duration` (`SoundBase.Duration` _mainsound))
  (add `AudioComponent.OnAudioPlaybackPercent` (`self.Audio`) (delegate `PlaybackChange`))
  (`AudioComponent.Play` _audio_2 0.0)
  (bind _asthird_person_character (cast `/Game/ThirdPersonBP/Blueprints/ThirdPersonCharacter` (`GameplayStatics.GetPlayerCharacter` 0) :!label _label))
  (bind _output_get (set `/Game/ThirdPersonBP/Blueprints/ThirdPersonCharacter.timeRemaining` (- (`self.Duration`) (`self.PlayedTime`)) _asthird_person_character))
  (if (<= _output_get 0.0)
    (bind _returnvalue_2 (`GameplayStatics.GetCurrentLevelName` true))
    (if (not (`KismetStringLibrary.EqualEqual_StrStr` _returnvalue_2 "Commissary"))
      (`WidgetBlueprintLibrary.SetInputMode_GameOnly` _returnvalue)
      (set `PlayerController.bShowMouseCursor` false _returnvalue)
      (bind _asgame_manager_2 (cast `/Game/GameManager` (`GameplayStatics.GetGameInstance`)))
      (bind _asthird_person_character_2 (cast `/Game/ThirdPersonBP/Blueprints/ThirdPersonCharacter` (`GameplayStatics.GetPlayerCharacter` 0)))
      (set `/Game/GameManager.playerCurrencyTotal` (+ (`/Game/GameManager.playerCurrencyTotal` _asgame_manager_2) (`/Game/ThirdPersonBP/Blueprints/ThirdPersonCharacter.CurrencyInLevel` _asthird_person_character_2)) _asgame_manager_2)
      (`GameplayStatics.OpenLevel` "Commissary"))
    (elif (`KismetSystemLibrary.K2_IsTimerActiveHandle` (`/Game/ThirdPersonBP/Blueprints/ThirdPersonCharacter.Timer` _asthird_person_character))
      (`AudioComponent.SetPaused` _audio_2 true)
      (else
        (set `self.unpauseTime` (stale `PlaybackChange` _output_get))
        (if (`AudioComponent.IsPlaying` _audio_2)
          (if (>= (`/Game/ThirdPersonBP/Blueprints/ThirdPersonCharacter.ipodBurnout` _asthird_person_character) 0.4)
            (`self.SetPitchMultiplier`)
            (`AudioComponent.SetPitchMultiplier` _audio (`self.PitchMultiplier`))
            (else
              (bind _output_get_2 (set `self.PitchMultiplier` 1.0))
              (`AudioComponent.SetPitchMultiplier` _audio _output_get_2))))))))

(event `self.ReceiveTick`
  (params (DeltaSeconds :type "Float (single-precision)"))
  (goto _label))

(event `PlaybackChange`
  (params (PlayingSoundWave :type "SoundWave Object Reference") (PlaybackPercent :type "Float (double-precision)"))
  (bind _output_get (set `self.PlayedTime` (* PlaybackPercent (`self.Duration`))))
  (for _array_element (`ConstantQNRT.GetNormalizedChannelConstantQAtTime` (`self.Constant_Ref`) (`self.PlayedTime`) 0)
    (bind _returnvalue (* _array_element 5.0))
    (if (and (> _returnvalue 0.0) (< _returnvalue 2.5))
      (`KismetMaterialLibrary.SetScalarParameterValue` "/Game/Emissive/Glow.Glow" "Emission" 100.0)
      (bind _asthird_person_character (cast `/Game/ThirdPersonBP/Blueprints/ThirdPersonCharacter` (`GameplayStatics.GetPlayerCharacter` 0)))
      (set `/Game/ThirdPersonBP/Blueprints/ThirdPersonCharacter.charOnBeat` true _asthird_person_character)
      (`KismetMaterialLibrary.SetScalarParameterValue` "/Game/Emissive/Glow_Beat/Glow_Collection.Glow_Collection" "Intensity" 75.0)
      (else
        (`KismetMaterialLibrary.SetScalarParameterValue` "/Game/Emissive/Glow.Glow" "Emission" 10.0)
        (bind _asthird_person_character_2 (cast `/Game/ThirdPersonBP/Blueprints/ThirdPersonCharacter` (`GameplayStatics.GetPlayerCharacter` 0)))
        (set `/Game/ThirdPersonBP/Blueprints/ThirdPersonCharacter.charOnBeat` false _asthird_person_character_2)
        (`KismetMaterialLibrary.SetScalarParameterValue` "/Game/Emissive/Glow_Beat/Glow_Collection.Glow_Collection" "Intensity" 50.0)))))

(fn `SetPitchMultiplier`
  (bind _asthird_person_character (cast `/Game/ThirdPersonBP/Blueprints/ThirdPersonCharacter` (`GameplayStatics.GetPlayerCharacter` 0)))
  (bind _ipodburnout (`/Game/ThirdPersonBP/Blueprints/ThirdPersonCharacter.ipodBurnout` _asthird_person_character))
  (if (>= _ipodburnout 0.9)
    (set `self.PitchMultiplier` 0.8)
    (elif (>= _ipodburnout 0.8)
      (set `self.PitchMultiplier` 0.85)
      (elif (>= _ipodburnout 0.7)
        (set `self.PitchMultiplier` 0.875)
        (elif (>= _ipodburnout 0.6)
          (set `self.PitchMultiplier` 0.9)
          (elif (>= _ipodburnout 0.5)
            (set `self.PitchMultiplier` 0.925)
            (elif (>= _ipodburnout 0.4)
              (set `self.PitchMultiplier` 0.95))))))))

(fn `UserConstructionScript`)